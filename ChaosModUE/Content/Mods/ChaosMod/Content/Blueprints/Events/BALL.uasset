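; BALL is a ChaosMod event actor: a randomly colored physics sphere that launches itself in a random direction when spawned.
; The construction script gives the sphere a dynamic instance of MAT_Balls, setting its Color to a random fully saturated, full-brightness hue.
; On BeginPlay, it applies a single large force to the sphere along a random unit vector.
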(event `self.ReceiveBeginPlay`
  (`PrimitiveComponent.AddForce` (`self.Sphere`) (* (`KismetMathLibrary.RandomUnitVector`) 100000.0) "None" false))

(fn `UserConstructionScript`
  (bind _returnvalue (`KismetMaterialLibrary.CreateDynamicMaterialInstance` "/Game/Mods/ChaosMod/Content/Materials/MAT_Balls.MAT_Balls"))
  (`PrimitiveComponent.SetMaterial` (`self.Sphere`) 0 _returnvalue)
  (`MaterialInstanceDynamic.SetVectorParameterValue` _returnvalue "Color" (`KismetMathLibrary.HSVToRGB` (`KismetMathLibrary.RandomFloatInRange` 0.0 360.0) 1.0 1.0)))